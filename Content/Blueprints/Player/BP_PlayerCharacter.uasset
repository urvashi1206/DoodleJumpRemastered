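; Player character for a 2D bouncing platformer that launches upward on begin play and again on every capsule hit.
; Jumps set the capsule's physics linear velocity directly rather than using the character jump.
; Each tick, the mouse's viewport half picks left or right, moving the actor along X without sweep and swapping the sprite flipbook.
; Falling faster than a threshold pauses the game and shows the end screen widget.
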(event OnComponentHit(CapsuleComponent)
  (params (HitComponent :type Primitive%20Component%20Object%20Reference) (OtherActor :type Actor%20Object%20Reference) (OtherComp :type Primitive%20Component%20Object%20Reference) (NormalImpulse :type Vector :default "0, 0, 0") (Hit :type Hit%20Result%20Structure%20%28by%20ref%29))
  ;[1 1 1] when hit platform, jump
  (CallFunction|JumpUp 7e+02))

(event Custom|JumpUp
  (params (Force :type Float%20%28double-precision%29))
  (Physics|SetPhysicsLinearVelocity (Variables|/Script/Engine.MovementComponent|GetUpdatedPrimitive (Variables|Character|GetCharacterMovement)) (Math|Vector|MakeVector 0.0 0.0 Force) false "None"))

(event EventBeginPlay
  (CallFunction|JumpUp 7e+02))

(event Collision|EventActorBeginOverlap
  (params (OtherActor :type Actor%20Object%20Reference)))

(event EventTick
  (params (DeltaSeconds :type Float%20%28single-precision%29))
  (bind _returnvalue (Transformation|GetActorLocation))
  (bind _sprite (Variables|Default|GetSprite))
  (if (< (.z (Transformation|GetComponentVelocity (Variables|Collision|GetCapsuleComponent))) -1e+03)
    (Game|SetGamePaused true)
    (bind _returnvalue_2 (UserInterface|CreateWidget "/Game/Blueprints/UI/HUD_EndScreen.HUD_EndScreen_C"))
    (UserInterface|Viewport|AddtoViewport _returnvalue_2 1)
    (else
      ;[1 1 1] Check mouse position
      (bind _returnvalue_3 (Class|WidgetLayoutLibrary|GetMousePositiononViewport))
      (if (<= (.x _returnvalue_3) (/ (.x (Viewport|GetViewportSize)) 2.0))
        ;[1 1 1] left
        (Transformation|SetActorLocation (+ _returnvalue (Math|Vector|MakeVector (* DeltaSeconds -4e+02) 0.0 0.0)) false false)
        (Sprite|SetFlipbook _sprite "/Game/Assets_Player/Player_FlipBookLeft.Player_FlipBookLeft")
        (else
          ;[1 1 1] right
          (Transformation|SetActorLocation (+ _returnvalue (Math|Vector|MakeVector (* DeltaSeconds 4e+02) 0.0 0.0)) false false)
          (Sprite|SetFlipbook _sprite "/Game/Assets_Player/Player_FlipBook_Right.Player_FlipBook_Right"))))))

(fn ConstructionScript)