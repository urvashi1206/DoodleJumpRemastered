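; Breakable one-way platform that crumbles after the player character hits it.
; Every Tick it reads player 0's vertical capsule velocity, enabling Box collision only while falling and disabling it otherwise.
; The RenderComponent animation is stopped on BeginPlay, then played when the player hits the platform, which destroys itself after a short delay.
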(event Collision|EventActorBeginOverlap
  (params (OtherActor :type Actor%20Object%20Reference)))

(event EventTick
  (params (DeltaSeconds :type Float%20%28single-precision%29))
  (bind _box (Variables|Default|GetBox))
  (bind _asbp_player_character (Utilities|Casting|CastToBP_PlayerCharacter (Game|GetPlayerCharacter 0)))
  (if (>= (.z (Transformation|GetComponentVelocity (Variables|/Script/Engine.Character|GetCapsuleComponent _asbp_player_character))) 0.0)
    (Collision|SetCollisionEnabled _box "NoCollision")
    (else
      (Collision|SetCollisionEnabled _box "QueryAndPhysics"))))

(event Collision|EventHit
  (params (MyComp :type Primitive%20Component%20Object%20Reference) (Other :type Actor%20Object%20Reference) (OtherComp :type Primitive%20Component%20Object%20Reference) (bSelfMoved :type Boolean) (HitLocation :type Vector :default "0, 0, 0") (HitNormal :type Vector :default "0, 0, 0") (NormalImpulse :type Vector :default "0, 0, 0") (Hit :type Hit%20Result%20Structure%20%28by%20ref%29))
  (Utilities|Casting|CastToBP_PlayerCharacter Other)
  (Audio|Components|Audio|Play (Variables|Default|GetRenderComponent))
  (Utilities|FlowControl|Delay 1.0)
  (Actor|DestroyActor))

(event EventBeginPlay
  (Audio|Components|Audio|Stop (Variables|Default|GetRenderComponent)))

(fn ConstructionScript)