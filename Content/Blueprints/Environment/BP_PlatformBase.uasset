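; BP_PlatformBase is a platform actor that the player can pass through while rising and collide with while falling.
; Each tick it reads the player capsule's vertical velocity and enables Box collision only when that velocity is negative.
; It also destroys itself once the player is 1000 or more units above it, cleaning up platforms left below.
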(event EventBeginPlay)

(event Collision|EventActorBeginOverlap
  (params (OtherActor :type Actor%20Object%20Reference)))

(event EventTick
  (params (DeltaSeconds :type Float%20%28single-precision%29))
  (bind _box (Variables|Default|GetBox))
  (bind _asbp_player_character (Utilities|Casting|CastToBP_PlayerCharacter (Game|GetPlayerCharacter 0)))
  (if (>= (- (.z (.location (Transformation|GetActorTransform _asbp_player_character))) (.z (.location (Transformation|GetActorTransform)))) 1e+03)
    (Actor|DestroyActor)
    (else
      ;[1 1 1] check if should have collisin
      (if (>= (.z (Transformation|GetComponentVelocity (Variables|/Script/Engine.Character|GetCapsuleComponent _asbp_player_character))) 0.0)
        (Collision|SetCollisionEnabled _box "NoCollision")
        (else
          (Collision|SetCollisionEnabled _box "QueryAndPhysics"))))))

(fn ConstructionScript)