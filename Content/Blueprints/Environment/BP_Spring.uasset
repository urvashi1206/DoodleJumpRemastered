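; BP_Spring is a spring that launches the player character upward when it is hit.
; A Box component hit casts to BP_PlayerCharacter, calls JumpUp with a fixed strength and plays FBSpring, which is stopped at BeginPlay.
; Unconnected logic that never runs would destroy the spring once the player is far above and toggle Box collision by vertical velocity.
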(event OnComponentHit(Box)
  (params (HitComponent :type Primitive%20Component%20Object%20Reference) (OtherActor :type Actor%20Object%20Reference) (OtherComp :type Primitive%20Component%20Object%20Reference) (NormalImpulse :type Vector :default "0, 0, 0") (Hit :type Hit%20Result%20Structure%20%28by%20ref%29))
  (bind _asbp_player_character (Utilities|Casting|CastToBP_PlayerCharacter OtherActor))
  (Development|PrintString "spring")
  (Default|JumpUp _asbp_player_character 1e+03)
  (Audio|Components|Audio|Play (Variables|Default|GetFB_Spring)))

(event EventBeginPlay
  (Audio|Components|Audio|Stop (Variables|Default|GetFB_Spring)))

(event Collision|EventActorBeginOverlap
  (params (OtherActor :type Actor%20Object%20Reference)))

(event EventTick
  (params (DeltaSeconds :type Float%20%28single-precision%29)))

(fn ConstructionScript)