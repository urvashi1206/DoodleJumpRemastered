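; BP_Bomb is a placed bomb that starts a countdown when the player character enters its box trigger.
; Overlap begin and end events track whether the player is in range, while timed delays swap the countdown sprite.
; When the countdown ends, it pauses the game and shows the end screen if the player is still in range, otherwise it destroys itself.
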(event OnComponentEndOverlap(Box)
  (params (OverlappedComponent :type Primitive%20Component%20Object%20Reference) (OtherActor :type Actor%20Object%20Reference) (OtherComp :type Primitive%20Component%20Object%20Reference) (OtherBodyIndex :type Integer))
  (Utilities|Casting|CastToBP_PlayerCharacter OtherActor)
  (Variables|Default|SetisPlayerInRange false))

(event OnComponentBeginOverlap(Box)
  (params (OverlappedComponent :type Primitive%20Component%20Object%20Reference) (OtherActor :type Actor%20Object%20Reference) (OtherComp :type Primitive%20Component%20Object%20Reference) (OtherBodyIndex :type Integer) (bFromSweep :type Boolean) (SweepResult :type Hit%20Result%20Structure%20%28by%20ref%29))
  (Utilities|Casting|CastToBP_PlayerCharacter OtherActor)
  (Variables|Default|SetisPlayerInRange true)
  (CallFunction|StartCountDown))

(event Custom|StartCountDown
  (Utilities|FlowControl|Delay 1.0)
  (Rendering|Components|Sprite|SetSprite (Variables|Default|GetCountDown) "/Game/Sprites_Doodle_Jump/game-tiles_Sprite_105.game-tiles_Sprite_105")
  (Utilities|FlowControl|Delay 1.0)
  (Rendering|Components|Sprite|SetSprite (Variables|Default|GetCountDown) "/Game/Sprites_Doodle_Jump/game-tiles_Sprite_104.game-tiles_Sprite_104")
  (Utilities|FlowControl|Delay 0.2)
  (if (Variables|Default|GetisPlayerInRange)
    (Game|SetGamePaused true)
    (bind _returnvalue (UserInterface|CreateWidget "/Game/Blueprints/UI/HUD_EndScreen.HUD_EndScreen_C"))
    (UserInterface|Viewport|AddtoViewport _returnvalue 2)
    (else
      (Actor|DestroyActor))))

(event EventBeginPlay)

(event Collision|EventActorBeginOverlap
  (params (OtherActor :type Actor%20Object%20Reference)))

(event EventTick
  (params (DeltaSeconds :type Float%20%28single-precision%29)))

(fn ConstructionScript)